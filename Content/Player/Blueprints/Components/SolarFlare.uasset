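; SolarFlare is a short-lived flare effect actor made of a Sphere mesh and a PointLight, which removes itself after playing.
; The construction script sets the sphere material's Intensity parameter to a high value.
; On BeginPlay, the Disappear timeline drives both the sphere's scale and the light's intensity from one track, then destroys the actor when it finishes.
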(event EventBeginPlay
  (bind _newtrack_0 (Timeline|Disappear Play)
    (:Update
      (Transformation|SetRelativeScale3D (Variables|Default|GetSphere) (* _newtrack_0 0.25))
      (Rendering|Components|Light|SetIntensity (Variables|Default|GetPointLight) (* _newtrack_0 1e+04)))
    (:Finished
      (Actor|DestroyActor))))

(event Collision|EventActorBeginOverlap
  (params (OtherActor :type Actor%20Object%20Reference)))

(event EventTick
  (params (DeltaSeconds :type Float%20%28single-precision%29)))

(fn ConstructionScript
  (Rendering|Material|SetScalarParameterValueonMaterials (Variables|Default|GetSphere) "Intensity" 5e+01))